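; Player character for a third-person shooter, with movement, spring-arm aim camera, weapon swapping, sliding and health.
; Enhanced Input drives the action functions; sliding hides the weapon, blocks aiming and firing, and ignores damage.
; Rifle and shotgun use randomized camera-origin line traces for point damage and spawn tracers, with shotgun pellets triggered by a montage notify.
; Death pulls the camera back, disables input, ragdolls with explosion effects and expires the actor.
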(event Input|EnhancedActionEvents|EnhancedInputActionIA_Jump
  (params (ActionValue :type Boolean) (ElapsedSeconds :type Float%20%28double-precision%29) (TriggeredSeconds :type Float%20%28double-precision%29) (InputAction :type Input%20Action%20Object%20Reference :default "/Game/Input/Actions/IA_Jump.IA_Jump"))
  ;[0.05098 0.05098 0.05098] ジャンプの処理
  (:Started
    (Character|Jump))
  (:Canceled
    (Character|StopJumping)))

(event Input|EnhancedActionEvents|EnhancedInputActionIA_Move
  (params (ActionValue :type Vector%202D%20Structure) (ElapsedSeconds :type Float%20%28double-precision%29) (TriggeredSeconds :type Float%20%28double-precision%29) (InputAction :type Input%20Action%20Object%20Reference :default "/Game/Input/Actions/IA_Move.IA_Move"))
  ;[0.05098 0.05098 0.05098] キャラクターの移動処理
  (CallFunction|OnMove (.x ActionValue) (.y ActionValue)))

(event Input|EnhancedActionEvents|EnhancedInputActionIA_Fire
  (params (ActionValue :type Boolean) (ElapsedSeconds :type Float%20%28double-precision%29) (TriggeredSeconds :type Float%20%28double-precision%29) (InputAction :type Input%20Action%20Object%20Reference :default "/Game/Input/Actions/IA_Fire.IA_Fire"))
  ;[0.05098 0.05098 0.05098] 銃の発砲処理
  (Utilities|OnFire))

(event Input|EnhancedActionEvents|EnhancedInputActionIA_Sliding
  (params (ActionValue :type Boolean) (ElapsedSeconds :type Float%20%28double-precision%29) (TriggeredSeconds :type Float%20%28double-precision%29) (InputAction :type Input%20Action%20Object%20Reference :default "/Game/Input/Actions/IA_Sliding.IA_Sliding"))
  ;[0.05098 0.05098 0.05098] スライディングの処理
  (Utilities|OnSliding))

(event Input|EnhancedActionEvents|EnhancedInputActionIA_Look
  (params (ActionValue :type Vector%202D%20Structure) (ElapsedSeconds :type Float%20%28double-precision%29) (TriggeredSeconds :type Float%20%28double-precision%29) (InputAction :type Input%20Action%20Object%20Reference :default "/Game/Input/Actions/IA_Look.IA_Look"))
  ;[0.05098 0.05098 0.05098] カメラ処理
  (CallFunction|OnLook (.x ActionValue) (.y ActionValue)))

(event Input|EnhancedActionEvents|EnhancedInputActionIA_Aiming
  (params (ActionValue :type Boolean) (ElapsedSeconds :type Float%20%28double-precision%29) (TriggeredSeconds :type Float%20%28double-precision%29) (InputAction :type Input%20Action%20Object%20Reference :default "/Game/Input/Actions/IA_Aiming.IA_Aiming"))
  ;[0.05098 0.05098 0.05098] 銃で狙う処理
  (:Triggered
    (CallFunction|OnAiming true))
  (:Completed
    (CallFunction|OnAiming false)))

(event EventBeginPlay
  ;[0.05098 0.05098 0.05098] ゲーム開始時の初期化処理
  (CallFunction|Init))

(event Game|Damage|EventAnyDamage
  (params (Damage :type Float%20%28single-precision%29) (DamageType :type Damage%20Type%20Object%20Reference) (InstigatedBy :type Controller%20Object%20Reference) (DamageCauser :type Actor%20Object%20Reference))
  ;[0.05098 0.05098 0.05098] ダメージを受けた時の処理
  (bind _dead (CallFunction|OnDamage Damage))
  (if _dead
    (CallFunction|OnDead)))

(fn ConstructionScript)

(fn Init
  (Variables|Default|SetLife 1e+02)
  (Variables|Default|SetIs%20Dead%20? false)
  (CallFunction|OnAiming false)
  (Collision|SetCollisionEnabled (Variables|Collision|GetCapsuleComponent) "QueryAndPhysics")
  (bind _asplayer_controller (Utilities|Casting|CastToPlayerController (Pawn|GetController)))
  (Utilities|IsValid (PlayerController|LocalPlayerSubsystems|GetEnhancedInputLocalPlayerSubsystem _asplayer_controller)
    (:Is%20Valid
      (Input|AddMappingContext (PlayerController|LocalPlayerSubsystems|GetEnhancedInputLocalPlayerSubsystem _asplayer_controller) "/Game/Input/IMC_Default.IMC_Default" 0 "(bIgnoreAllPressedKeysUntilRelease=True,bForceImmediately=False,bNotifyUserSettings=False)"))))

(fn OnMove
  (params (X :type Float%20%28double-precision%29) (Y :type Float%20%28double-precision%29))
  (bind _returnvalue (Pawn|GetControlRotation :!class /Script/Engine.Pawn))
  (if (not (Variables|Default|GetIs%20Dead%20?))
    (Pawn|Input|AddMovementInput (Math|Vector|GetRightVector (Math|Rotator|MakeRotator (.roll _returnvalue) 0.0 (.yaw _returnvalue))) X false)
    (Pawn|Input|AddMovementInput (Math|Vector|GetForwardVector (Math|Rotator|MakeRotator 0.0 0.0 (.yaw (Pawn|GetControlRotation :!class /Script/Engine.Pawn)))) Y false)))

(fn OnLook
  (params (X :type Float%20%28double-precision%29) (Y :type Float%20%28double-precision%29))
  ;[0.05098 0.05098 0.05098 1 14] 左右方向
  (Pawn|Input|AddControllerYawInput X)
  ;[0.05098 0.05098 0.05098 1 14] 上下方向
  (Pawn|Input|AddControllerPitchInput Y))

(fn OnAiming
  (params (Focus :type Boolean))
  (if (not (Variables|Default|GetIs%20Sliding%20?))
    (bind _output_get (Variables|Default|SetIs%20Focus%20? Focus))
    (if _output_get
      (CallFunction|SetViewPoint 9e+01 "0.000000,58.000000,70.000000" false true) ; 狙っている時
      (else
        (CallFunction|SetViewPoint 2.5e+02 "0.000000,80.000000,70.000000" false true) ; 通常時
      ))))

(fn OnDamage
  (params (Damage :type Float%20%28double-precision%29))
  (if (not (Variables|Default|GetIs%20Sliding%20?)) ; スライディング中は無敵
    (bind _output_get (Variables|Default|SetLife (- (Variables|Default|GetLife) Damage)))
    (bind _output_get_2 (Variables|Default|SetIs%20Dead%20? (<= _output_get 0.0)))
    (if _output_get_2
      (Variables|Default|SetLife 0.0))
    (return (Variables|Default|GetIs%20Dead%20?))))

(fn OnDead
  (bind _returnvalue (Transformation|GetActorLocation))
  (CallFunction|SetViewPoint 6e+02 "0.000000,0.000000,125.000000" false true)
  (Input|DisableInput (Game|GetPlayerController 0))
  (CallFunction|Ragdoll "0, 0, 0")
  (Effects|SpawnEmitteratLocation "/Game/Props/MilitaryWeapSilver/FX/Cascade/P_RocketLauncher_Explosion_01.P_RocketLauncher_Explosion_01" _returnvalue "0, 0, 0" "0.600000,0.600000,0.600000")
  (Audio|PlaySoundatLocation "/Game/Audio/SE/MS_OnPlayerIsDead.MS_OnPlayerIsDead" _returnvalue "0, 0, 0" 1.0 1.0 0.0 0 0 0 0)
  (Collision|SetCollisionEnabled (Variables|Collision|GetCapsuleComponent) "NoCollision")
  (Actor|SetLifeSpan 3.0))

(fn Ragdoll
  (params (Damage%20Direction :type Vector))
  (bind _mesh (Variables|Character|GetMesh))
  (bind _ragdollimpulsebone (LocalVariables|GetRagdollImpulseBone))
  (bind _charactermovement (Variables|Character|GetCharacterMovement))
  (bind _returnvalue (Pawn|Components|CharacterMovement|GetLastUpdateVelocity _charactermovement))
  (Collision|SetCollisionProfileName _mesh "Ragdoll" true :!class /Script/Engine.PrimitiveComponent)
  (Class|SkeletalMeshComponent|SetAllBodiesBelowSimulatePhysics _mesh _ragdollimpulsebone true true)
  (Physics|AddImpulse _mesh (+ (* (Math|Vector|Normalize Damage%20Direction) 1e+04) (+ _returnvalue (* (Math|Vector|Normalize _returnvalue) (LocalVariables|GetRagdoll%20Impulse%20Strength)))) _ragdollimpulsebone true))

(fn SetViewPoint
  (params (Target%20Arm%20Length :type Float%20%28single-precision%29) (Socket%20Offset :type Vector) (Orient%20Rotation%20to%20Movement :type Boolean) (Use%20Controller%20Rotation%20Yaw :type Boolean))
  (Variables|/Script/Engine.SpringArmComponent|SetTargetArmLength (Variables|Camera|GetCameraBoom) Target%20Arm%20Length)
  (Variables|/Script/Engine.SpringArmComponent|SetSocketOffset (Variables|Camera|GetCameraBoom) Socket%20Offset)
  (Variables|/Script/Engine.CharacterMovementComponent|SetbOrientRotationToMovement (Variables|Character|GetCharacterMovement) Orient%20Rotation%20to%20Movement)
  (Variables|Default|SetbUseControllerRotationYaw Use%20Controller%20Rotation%20Yaw))

(fn OnChangeWeapon
  (params (WeaponType :type E_WeaponType%20Enum :default "NewEnumerator0"))
  (bind _weapon (Variables|Default|GetWeapon))
  (bind _output_get (Variables|Default|SetEquippedWeapon WeaponType))
  (switch Utilities|FlowControl|Switch|SwitchonE_WeaponType _output_get
    (:NewEnumerator0
      (Components|SkeletalMesh|SetSkeletalMeshAsset _weapon "/Game/Props/MilitaryWeapSilver/Weapons/Assault_Rifle_A.Assault_Rifle_A")
      (Audio|PlaySound2D "/Game/Props/MilitaryWeapSilver/Sound/Rifle/Wavs/Rifle_AmmoPickup.Rifle_AmmoPickup" 1.0 1.0 0.0 0 0))
    (:NewEnumerator1
      (Components|SkeletalMesh|SetSkeletalMeshAsset _weapon "/Game/Props/MilitaryWeapSilver/Weapons/Shotgun_A.Shotgun_A")
      (Audio|PlaySound2D "/Game/Props/MilitaryWeapSilver/Sound/Shotgun/Wavs/Shotgun_AmmoPickup.Shotgun_AmmoPickup" 1.0 1.0 0.0 0 0))))

(fn OnFireAssultRifle
  (bind _followcamera (Variables|Camera|GetFollowCamera))
  (bind _returnvalue (Transformation|GetWorldLocation _followcamera))
  (Animation|PlayAnimMontage "/Game/Animations/Mannequin/Animations/Actions/AM_MM_Rifle_Fire.AM_MM_Rifle_Fire" 1.0 "None")
  (while (Math|Float|NearlyEqual(Float) (Class|AnimInstance|MontageGetPlayRate (Components|SkeletalMesh|GetAnimInstance (Variables|Character|GetMesh)) "/Game/Animations/Mannequin/Animations/Actions/AM_MM_Rifle_Fire.AM_MM_Rifle_Fire") 0.0 1e-06)
    _)
  (LocalVariables|SetSocketTransform (Transformation|GetSocketTransform (Variables|Default|GetWeapon) "MuzzleFlash" "RTS_World"))
  (Effects|SpawnEmitteratLocation "/Game/Props/MilitaryWeapSilver/FX/Cascade/P_AssaultRifle_MuzzleFlash.P_AssaultRifle_MuzzleFlash" (.location (LocalVariables|GetSocketTransform)) (.rotation (LocalVariables|GetSocketTransform)))
  (Audio|PlaySoundatLocation "/Game/Props/MilitaryWeapSilver/Sound/Rifle/Cues/RifleA_Fire_Cue.RifleA_Fire_Cue" (.location (LocalVariables|GetSocketTransform)) "0, 0, 0" 1.0 1.0 0.0 0 0 0 0)
  (if (Variables|Default|GetIs%20Focus%20?)
    (LocalVariables|SetDiffusion 0.02)
    (else
      (LocalVariables|SetDiffusion 0.02)))
  (LocalVariables|SetDiffusion (+ (LocalVariables|GetDiffusion) (Math|Float|MapRangeClamped (Math|Vector|VectorLength (Transformation|GetVelocity)) 0.0 4e+02 0.0 0.02)))
  (bind (_outhit _returnvalue_2) (Collision|LineTraceByChannel _returnvalue (+ _returnvalue (* (Math|Vector|Normalize (+ (Math|Vector|GetForwardVector (Transformation|GetWorldRotation _followcamera)) (Math|Vector|MakeVector (Math|Random|RandomFloatinRange (* (LocalVariables|GetDiffusion) -1.0) (LocalVariables|GetDiffusion)) (Math|Random|RandomFloatinRange (* (LocalVariables|GetDiffusion) -1.0) (LocalVariables|GetDiffusion)) (Math|Random|RandomFloatinRange (* (LocalVariables|GetDiffusion) -1.0) (LocalVariables|GetDiffusion))))) 5e+03)) "TraceTypeQuery1" false 0 "None"))
  (LocalVariables|SetHitResult _outhit)
  (Game|SpawnActorfromClass "/Game/Blueprints/BP_RifleTracer.BP_RifleTracer_C" (Math|Transform|MakeTransform (.location (LocalVariables|GetSocketTransform)) (Math|Rotator|FindLookatRotation (.location (LocalVariables|GetSocketTransform)) (.TraceEnd (Collision|BreakHitResult (LocalVariables|GetHitResult))))) "AlwaysSpawn" "MultiplyWithRoot" 0 (Variables|Default|GetTeam) 0)
  (if _returnvalue_2
    (Game|Damage|ApplyPointDamage (.HitActor (Collision|BreakHitResult (LocalVariables|GetHitResult))) 1e+01 (Math|Vector|Normalize (- (.Location (Collision|BreakHitResult (LocalVariables|GetHitResult))) (.TraceStart (Collision|BreakHitResult (LocalVariables|GetHitResult))))) (LocalVariables|GetHitResult))
    (Effects|SpawnEmitteratLocation "/Game/Props/StarterContent/Particles/P_Explosion.P_Explosion" (.Location (Collision|BreakHitResult (LocalVariables|GetHitResult))) "0, 0, 0" "0.300000,0.300000,0.300000")))

(fn OnFireShotGun
  (bind _followcamera (Variables|Camera|GetFollowCamera))
  (bind _returnvalue (Transformation|GetWorldLocation _followcamera))
  (LocalVariables|SetSocketTransform (Transformation|GetSocketTransform (Variables|Default|GetWeapon) "MuzzleFlash" "RTS_World"))
  (if (Variables|Default|GetIs%20Focus%20?)
    (LocalVariables|SetDiffusion 0.11)
    (else
      (LocalVariables|SetDiffusion 0.18)))
  (Effects|SpawnEmitteratLocation "/Game/Props/MilitaryWeapSilver/FX/Cascade/P_Shotgun_MuzzleFlash_01.P_Shotgun_MuzzleFlash_01" (.location (LocalVariables|GetSocketTransform)) (.rotation (LocalVariables|GetSocketTransform)))
  (Audio|PlaySound2D "/Game/Props/MilitaryWeapSilver/Sound/Shotgun/Cues/ShotgunA_Fire_Cue.ShotgunA_Fire_Cue" 1.0 1.0 0.0 0 0)
  (for _index (range 0 10)
    (if (Utilities|IsValid (Game|GetPlayerCharacter 0))
      (Game|SpawnActorfromClass "/Game/Blueprints/BP_RifleTracer.BP_RifleTracer_C" (Math|Transform|MakeTransform (.location (LocalVariables|GetSocketTransform)) (Math|Rotator|MakeRotationfromAxes (Math|Vector|Normalize (+ (Math|Vector|GetForwardVector (.rotation (LocalVariables|GetSocketTransform))) (Math|Vector|MakeVector (Math|Random|RandomFloatinRange (* (LocalVariables|GetDiffusion) -1.0) (LocalVariables|GetDiffusion)) (Math|Random|RandomFloatinRange (* (LocalVariables|GetDiffusion) -1.0) (LocalVariables|GetDiffusion)) (Math|Random|RandomFloatinRange (* (LocalVariables|GetDiffusion) -1.0) (LocalVariables|GetDiffusion))))) (Math|Vector|GetRightVector (.rotation (LocalVariables|GetSocketTransform))) (Math|Vector|GetUpVector (.rotation (LocalVariables|GetSocketTransform))))) "AlwaysSpawn" "MultiplyWithRoot" 0 (Variables|Default|GetTeam) 0)
      (bind (_outhit _returnvalue_2) (Collision|LineTraceByChannel _returnvalue (+ _returnvalue (* (Math|Vector|Normalize (+ (Math|Vector|GetForwardVector (.rotation (LocalVariables|GetSocketTransform))) (Math|Vector|MakeVector (Math|Random|RandomFloatinRange (* (LocalVariables|GetDiffusion) -1.0) (LocalVariables|GetDiffusion)) (Math|Random|RandomFloatinRange (* (LocalVariables|GetDiffusion) -1.0) (LocalVariables|GetDiffusion)) (Math|Random|RandomFloatinRange (* (LocalVariables|GetDiffusion) -1.0) (LocalVariables|GetDiffusion))))) 5e+03)) "TraceTypeQuery1" false 0 "None"))
      (LocalVariables|SetHitResult _outhit)
      (if _returnvalue_2
        (Game|Damage|ApplyPointDamage (.HitActor (Collision|BreakHitResult (LocalVariables|GetHitResult))) 15.0 (Math|Vector|Normalize (- (.Location (Collision|BreakHitResult (LocalVariables|GetHitResult))) (.TraceStart (Collision|BreakHitResult (LocalVariables|GetHitResult))))) (LocalVariables|GetHitResult))
        (Effects|SpawnEmitteratLocation "/Game/Props/StarterContent/Particles/P_Explosion.P_Explosion" (.Location (Collision|BreakHitResult (LocalVariables|GetHitResult))) "0, 0, 0" "0.300000,0.300000,0.300000")))))

(fn GetTeam
  (return (Variables|Default|GetTeam)))