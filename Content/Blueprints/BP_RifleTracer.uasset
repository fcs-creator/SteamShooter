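; BP_RifleTracer is a short-lived rifle tracer actor that damages what it hits and removes itself after a one-second lifetime.
; On Hit it applies point damage from AttackPower, spawns a scaled-down explosion emitter at the impact and destroys itself.
; An overlap-based damage path is present but disabled, leaving blocking hits as the damage trigger.
; GetTeam exposes its Team value, which the hit logic does not check.
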(event EventBeginPlay
  (Utilities|FlowControl|Delay 1.0)
  (Actor|DestroyActor))

(event Collision|EventActorBeginOverlap
  (params (OtherActor :type Actor%20Object%20Reference))
  (Game|Damage|ApplyDamage OtherActor (Variables|Default|GetAttack%20Power) 0 self)
  (Actor|DestroyActor))

(event Collision|EventHit
  (params (MyComp :type Primitive%20Component%20Object%20Reference) (Other :type Actor%20Object%20Reference) (OtherComp :type Primitive%20Component%20Object%20Reference) (bSelfMoved :type Boolean) (HitLocation :type Vector :default "0, 0, 0") (HitNormal :type Vector :default "0, 0, 0") (NormalImpulse :type Vector :default "0, 0, 0") (Hit :type Hit%20Result%20Structure%20%28by%20ref%29))
  (Game|Damage|ApplyPointDamage Other (Variables|Default|GetAttack%20Power) HitNormal Hit 0 self)
  (Effects|SpawnEmitteratLocation "/Game/Props/StarterContent/Particles/P_Explosion.P_Explosion" HitLocation "0, 0, 0" "0.300000,0.300000,0.300000")
  (Actor|DestroyActor))

(fn ConstructionScript)

(fn GetTeam
  (return (Variables|Default|GetTeam)))