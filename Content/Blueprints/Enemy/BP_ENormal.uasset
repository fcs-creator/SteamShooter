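; BP_ENormal is the normal enemy, a child Blueprint that sets its own green color, life and score value at BeginPlay.
; A looping timer with an interval randomized once at start calls Attack whenever the enemy is attackable.
; Attack runs the parent logic, then spawns a BP_BeamNormal at its location, rotated toward the found player and tagged with the enemy's Team.
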(event Custom|Fire
  (if (Variables|Default|GetIs%20Attackable%20?%20)
    (CallFunction|Attack)))

(event EventBeginPlay
  (|CallParentFunction)
  (CallFunction|SetColor "(R=0.000000,G=1.000000,B=0.040351,A=1.000000)")
  (bind _output_get (Variables|Default|SetLife 6e+01))
  (Variables|Default|SetMaxLife _output_get)
  (Variables|Default|SetScorePoint 1e+02)
  (Utilities|Time|SetTimerbyEvent (delegate Custom|Fire) (Math|Random|RandomFloatinRange 2.5 4.0) true))

(fn ConstructionScript
  (|CallParentFunction))

(fn Attack
  (bind _returnvalue (Transformation|GetActorTransform))
  (bind _location (Math|Transform|BreakTransform _returnvalue))
  (|CallParentFunction)
  (bind _player (CallFunction|FindPlayer))
  (if (Utilities|IsValid _player)
    (Game|SpawnActorfromClass "/Game/Blueprints/Enemy/BP_BeamNormal.BP_BeamNormal_C" (Math|Transform|MakeTransform _location (Math|Rotator|FindLookatRotation _location (Transformation|GetActorLocation _player))) "AlwaysSpawn" "MultiplyWithRoot" 0 (Variables|Default|GetTeam) 0)))

(fn GetTeam
  (return (Variables|Default|GetTeam)))