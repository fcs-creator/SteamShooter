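; Enemy that turns to face the player and periodically fires a shotgun-like burst of scattered beams.
; A looping timer with randomized interval and delay calls Fire when IsAttackable is set.
; Fire spawns multiple BP_BeamDiffusion actors, each with its forward vector randomly offset by Diffusion and tagged with the enemy's Team.
; Parent material overrides also tint the Cylinder mesh through its own dynamic material, keeping that mesh's glow at zero.
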(event Custom|Fire
  (bind _diffusion (Variables|Default|GetDiffusion))
  (bind _capsulecomponent (Variables|Default|GetCapsuleComponent))
  (bind _returnvalue (Transformation|GetWorldRotation _capsulecomponent))
  (bind _returnvalue_2 (* _diffusion -1.0))
  (if (not (Variables|Default|GetHas%20Fire%20Start%20?))
    (Variables|Default|SetHas%20Fire%20Start%20? true)
    (Utilities|FlowControl|ForLoopwithBreak 0 10
      (:LoopBody
        (if (Utilities|IsValid (Game|GetPlayerCharacter 0))
          (Game|SpawnActorfromClass "/Game/Blueprints/Enemy/BP_BeamDiffusion.BP_BeamDiffusion_C" (Math|Transform|MakeTransform (.Location (Math|Transform|BreakTransform (Transformation|GetActorTransform))) (Math|Rotator|MakeRotationfromAxes (Math|Vector|Normalize (+ (Math|Vector|GetForwardVector _returnvalue) (Math|Vector|MakeVector (Math|Random|RandomFloatinRange _returnvalue_2 _diffusion) (Math|Random|RandomFloatinRange _returnvalue_2 _diffusion) (Math|Random|RandomFloatinRange _returnvalue_2 _diffusion)))) (Math|Vector|GetRightVector _returnvalue) (Math|Vector|GetUpVector _returnvalue))) "AlwaysSpawn" "MultiplyWithRoot" 0 (Variables|Default|GetTeam) 0)))
      (:Completed
        (Variables|Default|SetHas%20Fire%20Start%20? false)))))

(event Custom|OnFire
  (Utilities|FlowControl|Delay (Math|Random|RandomFloatinRange 0.5 1.0))
  (if (Variables|Default|GetIs%20Attackable%20?%20)
    (CallFunction|Fire)))

(event EventBeginPlay
  (|CallParentFunction)
  (CallFunction|SetColor "(R=1.000000,G=0.896270,B=0.000000,A=1.000000)")
  (bind _output_get (Variables|Default|SetLife 7e+01))
  (Variables|Default|SetMaxLife _output_get)
  (Variables|Default|SetScorePoint 2e+02)
  (Variables|Default|SetDiffusion 0.2)
  (Utilities|Time|SetTimerbyEvent (delegate Custom|OnFire) (Math|Random|RandomFloatinRange 1.5 2.0) true))

(event EventTick
  (params (DeltaSeconds :type Float%20%28single-precision%29))
  (CallFunction|LookatPlayer))

(fn ConstructionScript
  (|CallParentFunction))

(fn CreateDynamicMaterialInstance
  (bind _cylinder (Variables|Default|GetCylinder))
  (|CallParentFunction)
  (bind _returnvalue (Rendering|Material|CreateDynamicMaterialInstance _cylinder 0 (Rendering|Material|GetMaterial _cylinder 0) "None" :!class /Script/Engine.PrimitiveComponent))
  (Variables|Default|SetMID2 _returnvalue))

(fn SetColor
  (params (Color :type Linear%20Color%20Structure))
  (|CallParentFunction Color)
  (Rendering|Material|SetVectorParameterValue (Variables|Default|GetMID2) "BaseColor" Color :!class /Script/Engine.MaterialInstanceDynamic))

(fn SetEmissive
  (params (Glow :type Float%20%28double-precision%29))
  (|CallParentFunction Glow)
  (Rendering|Material|SetScalarParameterValue (Variables|Default|GetMID2) "GlowAmount" 0.0 :!class /Script/Engine.MaterialInstanceDynamic))

(fn GetTeam
  (return (Variables|Default|GetTeam)))