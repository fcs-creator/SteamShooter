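; BP_ERapid is a blue-tinted enemy that faces the player and fires rapid three-shot beam bursts.
; It extends a parent Blueprint, setting its own color, life and score value on BeginPlay.
; While attackable, a randomized Delay on Tick paces Fire, which starts a looping timer guarded against re-entry.
; Each timer tick spawns a team-tagged BP_BeamRapid aimed at the player, clearing itself after the third shot.
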(event Custom|Fire
  (if (not (Variables|Default|GetHas%20Fire%20Start%20?))
    (Variables|Default|SetHas%20Fire%20Start%20? true)
    (Variables|Default|SetShotCount 0)
    (bind _returnvalue (Utilities|Time|SetTimerbyEvent (delegate Custom|Shot) 0.1 true))
    (Variables|Default|SetFireTimer _returnvalue)))

(event Custom|Shot
  (bind _returnvalue (Transformation|GetActorTransform))
  (bind _returnvalue_2 (Game|GetPlayerCharacter 0))
  (bind _location (Math|Transform|BreakTransform _returnvalue))
  (bind _result (Math|Integer|IncrementInt (Variables|Default|GetShotCount))
    (:%20%20
      (Variables|Default|SetShotCount _result)
      (if (Utilities|IsValid _returnvalue_2)
        (Game|SpawnActorfromClass "/Game/Blueprints/Enemy/BP_BeamRapid.BP_BeamRapid_C" (Math|Transform|MakeTransform _location (Math|Rotator|FindLookatRotation _location (Transformation|GetActorLocation _returnvalue_2))) "AlwaysSpawn" "MultiplyWithRoot" 0 (Variables|Default|GetTeam) 0)
        (if (>= (Variables|Default|GetShotCount) 3)
          (Variables|Default|SetHas%20Fire%20Start%20? false)
          (Utilities|Time|ClearandInvalidateTimerbyHandle (Variables|Default|GetFireTimer)))))))

(event EventBeginPlay
  (|CallParentFunction)
  (CallFunction|SetColor "(R=0.000000,G=0.147027,B=1.000000,A=1.000000)")
  (bind _output_get (Variables|Default|SetLife 5e+01))
  (Variables|Default|SetMaxLife _output_get)
  (Variables|Default|SetScorePoint 3e+02))

(event EventTick
  (params (DeltaSeconds :type Float%20%28single-precision%29))
  (CallFunction|LookatPlayer)
  (if (Variables|Default|GetIs%20Attackable%20?%20)
    (Utilities|FlowControl|Delay (Math|Random|RandomFloatinRange 1.5 3.0))
    (CallFunction|Fire)))

(fn ConstructionScript
  (|CallParentFunction))

(fn GetTeam
  (return (Variables|Default|GetTeam)))