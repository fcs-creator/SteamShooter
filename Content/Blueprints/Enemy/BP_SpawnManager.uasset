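; Enemy spawn manager that fills the level at BeginPlay and keeps the live enemy count topped up to a fixed target.
; Construction loads enemy rows from DT_Enemies, and BeginPlay gathers BP_SpawnAnchor actors as spawn points.
; Each spawn picks a class by AppearanceRate-weighted random roll and places it at a random anchor.
; DeadEnemy lowers the count, letting Tick respawn after a random delay; the equal-rate picker is unused.
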(event EventBeginPlay
  (Variables|Default|SetSpawnNum 12)
  (bind _outactors (Actor|GetAllActorsOfClass "/Game/Blueprints/Enemy/BP_SpawnAnchor.BP_SpawnAnchor_C"))
  (Variables|Default|SetAnchors _outactors)
  (CallFunction|SpawnEnemies))

(event EventTick
  (params (DeltaSeconds :type Float%20%28single-precision%29))
  (if (< (Variables|Default|GetCurrentSpawnNum) (Variables|Default|GetSpawnNum))
    (Utilities|FlowControl|Delay (Math|Random|RandomFloatinRange 1.0 2.0))
    (CallFunction|SpawnEnemy)))

(fn ConstructionScript
  (CallFunction|GetDataTableValue))

(fn GetDataTableValue
  (bind _outrownames (DataTable|GetDataTableRowNames "/Game/Blueprints/Enemy/Data/DT_Enemies.DT_Enemies"))
  (for _array_element _outrownames
    (bind _returnvalue (Utilities|GetDataTableRow "/Game/Blueprints/Enemy/Data/DT_Enemies.DT_Enemies" _array_element)
      (:then
        (Utilities|Array|AddUnique (Variables|Default|GetEnemies) _returnvalue)))))

(fn SpawnEnemies
  (Variables|Default|SetAnchorNum (Utilities|Array|Length (Variables|Default|GetAnchors)))
  (for _index (range 0 (- (Variables|Default|GetSpawnNum) 1))
    (CallFunction|SpawnEnemy)))

(fn SpawnEnemy
  (bind _result (Math|Integer|IncrementInt (Variables|Default|GetCurrentSpawnNum))
    (:%20%20
      (Variables|Default|SetCurrentSpawnNum _result)
      (bind _enemy_class (CallFunction|ChooseEnemybyAppearanceRate))
      (Game|SpawnActorfromClass _enemy_class (Math|Transform|MakeTransform (CallFunction|ChooseAnchor) "0, 0, 0" "1.000000,1.000000,1.000000") "AlwaysSpawn" "MultiplyWithRoot" 0 0))))

(fn DeadEnemy
  (bind _result (Math|Integer|DecrementInt (Variables|Default|GetCurrentSpawnNum))
    (:%20%20
      (if (<= _result 0)
        (Variables|Default|SetCurrentSpawnNum 0)))))

(fn ChooseEnemybyAppearanceRate
  (Variables|Default|SetTotalAppearanceRate 0.0)
  (for _array_element (Variables|Default|GetEnemies)
    (Variables|Default|SetTotalAppearanceRate (+ (.AppearanceRate (Utilities|Struct|BreakST_Enemy _array_element)) (Variables|Default|GetTotalAppearanceRate))))
  (Variables|Default|SetRandomPoint (* (Variables|Default|GetTotalAppearanceRate) (Math|Random|RandomFloat)))
  (for _array_element_2 (Variables|Default|GetEnemies)
    (if (< (Variables|Default|GetRandomPoint) (.AppearanceRate (Utilities|Struct|BreakST_Enemy _array_element_2))) ; RandomPointを出現率と比較
      (return (.Class (Utilities|Struct|BreakST_Enemy _array_element_2))) ; 出現率より低いならば出現
      (else
        (Variables|Default|SetRandomPoint (- (Variables|Default|GetRandomPoint) (.AppearanceRate (Utilities|Struct|BreakST_Enemy _array_element_2)))) ; 出現率より高いならば出現率をマイナス
      ))))

(fn ChooseEnemybyEqualRate
  (bind _enemies (Variables|Default|GetEnemies))
  (return (.Class (Utilities|Struct|BreakST_Enemy (Utilities|Array|Get(acopy) _enemies (Math|Random|RandomIntegerinRange 0 (- (Utilities|Array|Length _enemies) 1)))))))

(fn ChooseAnchor
  (return (Transformation|GetActorLocation (Utilities|Array|Get(acopy) (Variables|Default|GetAnchors) (Math|Random|RandomIntegerinRange 0 (- (Variables|Default|GetAnchorNum) 1))))))