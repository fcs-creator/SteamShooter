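; BP_Enemy is an enemy actor, apparently a base class given its empty Attack, that takes point damage and awards score on death.
; Damage drives a dynamic material's glow by remaining life; death triggers explosion, sound, score via BP_GameMode and destruction, which notifies BP_SpawnManager.
; The HUD time-up event clears IsAttackable.
; Uncalled helpers provide recoloring, interpolated facing toward the player and opposing-team lookup through BPI_Team.
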(event Custom|OnTimeUpEvent
  (Variables|Default|SetIs%20Attackable%20?%20 false))

(event Custom|OnDestoryed
  (params (DestroyedActor :type Actor%20Object%20Reference))
  (bind _outactors (Actor|GetAllActorsOfClass "/Game/Blueprints/Enemy/BP_SpawnManager.BP_SpawnManager_C")) ; スポーンマネージャに知らせる
  (Utilities|IsValid (Utilities|Array|Get(acopy) _outactors)
    (:Is%20Valid
      (Default|DeadEnemy (Utilities|Array|Get(acopy) _outactors)))))

(event Game|Damage|EventPointDamage
  (params (Damage :type Float%20%28single-precision%29) (DamageType :type Damage%20Type%20Object%20Reference) (HitLocation :type Vector :default "0, 0, 0") (HitNormal :type Vector :default "0, 0, 0") (HitComponent :type Primitive%20Component%20Object%20Reference) (BoneName :type Name :default "None") (ShotFromDirection :type Vector :default "0, 0, 0") (InstigatedBy :type Controller%20Object%20Reference) (DamageCauser :type Actor%20Object%20Reference) (HitInfo :type Hit%20Result%20Structure%20%28by%20ref%29))
  (bind _dead (CallFunction|OnDamage Damage))
  (if _dead
    (CallFunction|OnDead)
    (CallFunction|AddScore)
    (Actor|DestroyActor)))

(event EventBeginPlay
  (Variables|Default|SetIs%20Attackable%20?%20 true)
  (CallFunction|CreateDynamicMaterialInstance)
  (Utilities|FlowControl|Delay 0.2)
  (bind _asbp_game_mode (Utilities|Casting|CastToBP_GameMode (Game|GetGameMode)))
  (EventDispatchers|BindEventtoOnTimeUp (Variables|/Game/Blueprints/BP_GameMode.BP_GameMode_C|GetHUD _asbp_game_mode) (delegate Custom|OnTimeUpEvent))
  (Game|BindEventtoOnDestroyed (delegate Custom|OnDestoryed)))

(fn ConstructionScript)

(fn Attack)

(fn FindPlayer
  (bind _outactors (Actor|GetAllActorswithInterface "/Game/Blueprints/BPI_Team.BPI_Team_C"))
  (for _array_element _outactors
    (bind _team (Class|BPITeam|GetTeam(Message) _array_element))
    (if (Utilities|Enum|NotEqual(Enum) _team (Variables|Default|GetTeam))
      (return _array_element))))

(fn OnDamage
  (params (Damage :type Float%20%28double-precision%29))
  (bind _output_get (Variables|Default|SetLife (- (Variables|Default|GetLife) Damage)))
  (if (<= _output_get 0.0)
    (Variables|Default|SetLife 0.0))
  (CallFunction|SetEmissive (Math|Float|MapRangeClamped (/ (Variables|Default|GetLife) (Variables|Default|GetMaxLife)) 1.0 0.0 0.0 1e+02)) ; 体力が減るほど光るようにする
  (return (<= _output_get 0.0)))

(fn OnDead
  (bind _returnvalue (Transformation|GetActorLocation))
  (Effects|SpawnEmitteratLocation "/Game/Props/MilitaryWeapSilver/FX/Cascade/P_Grenade_Explosion_01.P_Grenade_Explosion_01" _returnvalue "0, 0, 0" "0.500000,0.500000,0.500000")
  (Audio|PlaySoundatLocation "/Game/Audio/SE/MS_OnEnemyIsDead.MS_OnEnemyIsDead" _returnvalue "0, 0, 0" 1.0 1.0 0.0 0 0 0 0))

(fn AddScore
  (bind _asbp_game_mode (Utilities|Casting|CastToBP_GameMode (Game|GetGameMode)))
  (Default|AddScore _asbp_game_mode true (Variables|Default|GetScorePoint)))

(fn CreateDynamicMaterialInstance
  (bind _staticmesh (Variables|Default|GetStaticMesh))
  (bind _returnvalue (Rendering|Material|CreateDynamicMaterialInstance _staticmesh 0 (Rendering|Material|GetMaterial _staticmesh 0) "None" :!class /Script/Engine.PrimitiveComponent))
  (Variables|Default|SetMID _returnvalue))

(fn SetColor
  (params (Color :type Linear%20Color%20Structure))
  (Rendering|Material|SetVectorParameterValue (Variables|Default|GetMID) "BaseColor" Color :!class /Script/Engine.MaterialInstanceDynamic))

(fn SetEmissive
  (params (Glow :type Float%20%28double-precision%29))
  (Rendering|Material|SetScalarParameterValue (Variables|Default|GetMID) "GlowAmount" Glow :!class /Script/Engine.MaterialInstanceDynamic))

(fn LookatPlayer
  (bind _returnvalue (Game|GetPlayerCharacter 0))
  (Utilities|IsValid _returnvalue
    (:Is%20Valid
      (Transformation|SetActorRotation (Math|Interpolation|RInterpTo (Transformation|GetActorRotation) (Math|Rotator|FindLookatRotation (Transformation|GetActorLocation) (Transformation|GetActorLocation _returnvalue)) (Utilities|Time|GetWorldDeltaSeconds) 5.0)))))

(fn GetTeam
  (return (Variables|Default|GetTeam)))