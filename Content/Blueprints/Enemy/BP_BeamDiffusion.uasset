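; BP_BeamDiffusion is a short-lived beam projectile in the Enemy folder that damages actors of another team.
; On BeginPlay it plays a firing sound, then destroys itself after a half-second delay if it has not struck a target.
; On Hit it compares the other actor's team to its own, and on a mismatch applies damage, spawns a metal impact effect and destroys itself.
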(event EventBeginPlay
  (Audio|PlaySoundatLocation "/Game/Audio/SE/MS_Beam.MS_Beam" (Transformation|GetActorLocation) "0, 0, 0" 0.3 1.0 0.0 0 0 0 0) ; 発射音
  (Utilities|FlowControl|Delay 0.5) ; 当たらなかった場合は消す
  (Actor|DestroyActor))

(event Collision|EventHit
  (params (MyComp :type Primitive%20Component%20Object%20Reference) (Other :type Actor%20Object%20Reference) (OtherComp :type Primitive%20Component%20Object%20Reference) (bSelfMoved :type Boolean) (HitLocation :type Vector :default "0, 0, 0") (HitNormal :type Vector :default "0, 0, 0") (NormalImpulse :type Vector :default "0, 0, 0") (Hit :type Hit%20Result%20Structure%20%28by%20ref%29))
  (bind _team (Class|BPITeam|GetTeam(Message) Other))
  (if (Utilities|Enum|NotEqual(Enum) _team (Variables|Default|GetTeam))
    (Game|Damage|ApplyDamage Other 5.0 0 self)
    (Effects|SpawnEmitteratLocation "/Game/Props/MilitaryWeapSilver/FX/Cascade/P_Impact_Metal_Medium_01.P_Impact_Metal_Medium_01" HitLocation)
    (Actor|DestroyActor)))

(fn ConstructionScript)

(fn GetTeam
  (return (Variables|Default|GetTeam)))