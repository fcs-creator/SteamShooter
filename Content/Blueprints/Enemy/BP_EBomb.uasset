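; BP_EBomb is a bomb enemy that sets life and score on spawn and detonates after a timed warning.
; Its Explosion event, if the bomb is attackable, turns it red and starts a one-second looping Alert timer only once.
; The first three alerts play a warning sound and pulse emissive through a timeline.
; Tick polls the alert count and on the fourth spawns effects, applies radial damage and destroys the actor.
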(event Custom|Explosion
  (if (Variables|Default|GetIs%20Attackable%20?%20)
    (if (not (Variables|Default|Gethas%20Alert%20Start%20?))
      (Variables|Default|Sethas%20Alert%20Start%20? true)
      (bind _returnvalue (Utilities|Time|SetTimerbyEvent (delegate Custom|Alert) 1.0 true))
      (Variables|Default|SetAlertTimer _returnvalue)
      (CallFunction|SetColor "(R=1.000000,G=0.000000,B=0.035222,A=1.000000)"))))

(event Custom|Alert
  (bind _result (Math|Integer|IncrementInt (Variables|Default|GetAlertCount))
    (:%20%20
      (bind _output_get (Variables|Default|SetAlertCount _result))
      (if (<= _output_get 3)
        (Audio|PlaySoundatLocation "/Game/Audio/SE/MS_WarningSilen.MS_WarningSilen" (Transformation|GetActorLocation) "0, 0, 0" 2.0 1.0 0.0 0 0 0 0)
        (bind _glow (Timeline|タイムライン PlayFromStart)
          (:Update
            (CallFunction|SetEmissive _glow)))))))

(event EventBeginPlay
  (|CallParentFunction)
  (CallFunction|SetColor "(R=1.000000,G=0.391573,B=0.000000,A=1.000000)")
  (bind _output_get (Variables|Default|SetLife 1.8e+02))
  (Variables|Default|SetMaxLife _output_get)
  (Variables|Default|SetScorePoint 5e+02)
  (Variables|Default|SetAlertCount 0))

(event EventTick
  (params (DeltaSeconds :type Float%20%28single-precision%29))
  (bind _returnvalue (Transformation|GetActorLocation))
  (if (>= (Variables|Default|GetAlertCount) 4)
    (Effects|SpawnEmitteratLocation "/Game/Props/MilitaryWeapSilver/FX/Cascade/P_RocketLauncher_Explosion_01.P_RocketLauncher_Explosion_01" _returnvalue "0, 0, 0" "1.300000,1.300000,1.300000")
    (Audio|PlaySoundatLocation "/Game/Audio/SE/MS_Explosion.MS_Explosion" _returnvalue "0, 0, 0" 1.5 1.0 0.0 0 0 0 0)
    (Game|Damage|ApplyRadialDamage 1e+02 _returnvalue 5e+02 0 0 0 0 false "ECC_Visibility")
    (Actor|DestroyActor)))

(fn ConstructionScript
  (|CallParentFunction))

(fn GetTeam
  (return (Variables|Default|GetTeam)))