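; Rare purple, glowing enemy with a high score value that warps around the arena and removes itself if left alive.
; BeginPlay sets stats, warps once, then starts a timer whose flag-guarded Warp event begins a looping Move timer at one random interval.
; Each Move teleports to a random point, spawns an impact effect at a separately randomized point, and destroys the actor after five timed warps.
; OnDamage reapplies the glow after parent handling.
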(event Custom|OnWarp
  (if (not (Variables|Default|GetHas%20Start%20Warp%20%20?))
    (Variables|Default|SetHas%20Start%20Warp%20%20? true)
    (Variables|Default|SetWarpCount 0)
    (bind _returnvalue (Utilities|Time|SetTimerbyEvent (delegate Custom|Move) (Math|Random|RandomFloatinRange 3.0 6.0) true))
    (Variables|Default|SetWarpTimer _returnvalue)))

(event Custom|Move
  (bind _returnvalue (Math|Random|RandomFloatinRange -2e+03 2e+03))
  (bind _returnvalue_2 (Math|Random|RandomFloatinRange -2e+03 2e+03))
  (bind _returnvalue_3 (Math|Random|RandomFloatinRange 4e+02 8e+02))
  (bind _returnvalue_4 (Math|Vector|MakeVector _returnvalue_2 _returnvalue _returnvalue_3))
  (bind _result (Math|Integer|IncrementInt (Variables|Default|GetWarpCount))
    (:%20%20
      (Variables|Default|SetWarpCount _result)
      (Transformation|SetActorLocation _returnvalue_4 true true)
      (Effects|SpawnEmitteratLocation "/Game/Props/MilitaryWeapSilver/FX/Cascade/P_Impact_Metal_Medium_01.P_Impact_Metal_Medium_01" _returnvalue_4)
      (if (>= (Variables|Default|GetWarpCount) 5)
        (Variables|Default|SetHas%20Start%20Warp%20%20? false)
        (Utilities|Time|ClearandInvalidateTimerbyHandle (Variables|Default|GetWarpTimer))
        (Actor|DestroyActor)))))

(event Custom|Warp
  (CallFunction|OnWarp))

(event EventBeginPlay
  (|CallParentFunction)
  (CallFunction|SetColor "(R=0.564712,G=0.000000,B=1.000000,A=1.000000)")
  (CallFunction|SetEmissive 2e+03)
  (bind _output_get (Variables|Default|SetLife 1.2e+02))
  (Variables|Default|SetMaxLife _output_get)
  (Variables|Default|SetScorePoint 5e+03)
  (CallFunction|Move)
  (Utilities|Time|SetTimerbyEvent (delegate Custom|Warp) 2.0 true))

(fn ConstructionScript
  (|CallParentFunction))

(fn OnDamage
  (params (Damage :type Float%20%28double-precision%29))
  (bind _dead (|CallParentFunction Damage))
  (CallFunction|SetEmissive 2e+03)
  (return _dead))