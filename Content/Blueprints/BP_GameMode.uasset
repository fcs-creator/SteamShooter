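; Game mode for a timed score-attack game that manages the HUD, combo scoring, player respawn and the end-of-time result screen.
; AddScore multiplies points by the combo, which grows on destroys and resets in Tick after a time window that shrinks as it climbs.
; Player destruction spawns and possesses a new BP_Player, rebinds the event and applies a HUD time penalty.
; The HUD's time-up event freezes scoring and passes the score to the result ranking.
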(event Custom|OnDestroyedEvent
  (params (DestroyedActor :type Actor%20Object%20Reference))
  (bind _respawn_actor (CallFunction|Respawn))
  (Game|BindEventtoOnDestroyed _respawn_actor (delegate Custom|OnDestroyedEvent)))

(event Custom|OnTimeUpEvent
  (CallFunction|OnTimeUp))

(event EventBeginPlay
  (CallFunction|InitGame)
  (EventDispatchers|BindEventtoOnTimeUp (Variables|Default|GetHUD) (delegate Custom|OnTimeUpEvent))
  (Game|BindEventtoOnDestroyed (Game|Player|GetPlayerPawn 0) (delegate Custom|OnDestroyedEvent)))

(event EventTick
  (params (DeltaSeconds :type Float%20%28single-precision%29))
  (CallFunction|UpdateCombo DeltaSeconds))

(fn ConstructionScript)

(fn InitGame
  (Variables|Default|SetComboLimitTime 1e+01)
  (Variables|Default|SetCombo 0)
  (Variables|Default|SetIs%20TimeUp? false)
  (CallFunction|CreateHUD))

(fn CreateHUD
  (Utilities|FlowControl|Sequence
    (:then_0
      (bind _returnvalue (UserInterface|CreateWidget "/Game/UI/WBP_HUD.WBP_HUD_C"))
      (bind _output_get (Variables|Default|SetHUD _returnvalue))
      (UserInterface|Viewport|AddtoViewport _output_get 0))
    (:then_1
      (bind _returnvalue_2 (UserInterface|CreateWidget "/Game/UI/WBP_Result.WBP_Result_C"))
      (Variables|Default|SetResult _returnvalue_2))))

(fn Respawn
  (bind _hud (Variables|Default|GetHUD))
  (Default|IncreseReduceAmountTime _hud)
  (Default|ShowMinusTime _hud)
  (bind _returnvalue (Game|SpawnActorfromClass "/Game/Blueprints/BP_Player.BP_Player_C" (Transformation|GetActorTransform (Class|GameModeBase|FindPlayerStart)) "AlwaysSpawn" "MultiplyWithRoot" 0 0)) ; キャラクターを指定の場所にスポーンさせる：戻り値がスポーンしたキャラクター
  (Pawn|Possess (Game|GetPlayerController 0) _returnvalue) ; リスポーンしたキャラクターを操作できるように設定
  (return _returnvalue))

(fn AddScore
  (params (Destroy :type Boolean) (Value :type Float%20%28double-precision%29))
  (if (not (Variables|Default|GetIs%20TimeUp?))
    (if Destroy
      (Variables|Default|SetIs%20Combo%20? true)
      (bind _result (Math|Integer|IncrementInt (Variables|Default|GetCombo))
        (:%20%20
          (bind _output_get (Variables|Default|SetCombo _result))
          (Variables|Default|SetComboLimitTime (Math|Float|MapRangeClamped (Math|Conversions|ToFloat(Integer) _output_get) 1.0 3e+01 7.0 2.0))
          (Variables|Default|SetComboErapsedTime 0.0))))
    (bind _output_get_2 (Variables|Default|SetScore (+ (Variables|Default|GetScore) (* Value (Variables|Default|GetCombo)))))
    (if (> _output_get_2 0.0)
      _
      (else
        (Variables|Default|SetScore 0.0)))
    (Rendering|Components|TextRender|SetText (Variables|/Game/UI/WBP_HUD.WBP_HUD_C|GetScore (Variables|Default|GetHUD)) (Utilities|Text|ToText(Integer) (Math|Float|Truncate (Variables|Default|GetScore)) false false 8))))

(fn UpdateCombo
  (params (DeltaSeconds :type Float%20%28double-precision%29))
  (Rendering|Components|TextRender|SetText (Variables|/Game/UI/WBP_HUD.WBP_HUD_C|GetCombo (Variables|Default|GetHUD)) (Utilities|Text|ToText(String) (Utilities|String|Append "Combo " (Utilities|String|ToString(Integer) (Variables|Default|GetCombo)))))
  (Progress|SetPercent (Variables|/Game/UI/WBP_HUD.WBP_HUD_C|GetComboLimitTime (Variables|Default|GetHUD)) (/ (- (Variables|Default|GetComboLimitTime) (Variables|Default|GetComboErapsedTime)) (Variables|Default|GetComboLimitTime)))
  (if (Variables|Default|GetIs%20Combo%20?)
    (bind _output_get (Variables|Default|SetComboErapsedTime (+ DeltaSeconds (Variables|Default|GetComboErapsedTime))))
    (if (> _output_get (Variables|Default|GetComboLimitTime))
      (Variables|Default|SetIs%20Combo%20? false)
      (Variables|Default|SetComboErapsedTime 0.0)
      (Variables|Default|SetCombo 0))))

(fn OnTimeUp
  (bind _result (Variables|Default|GetResult))
  (Variables|Default|SetIs%20TimeUp? true)
  (Widget|RemovefromParent (Variables|Default|GetHUD))
  (UserInterface|Viewport|AddtoViewport _result 0)
  (Default|UpdateRanking _result (Math|Float|Truncate (Variables|Default|GetScore))))