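; BP_ChangeWeapon is a weapon-change item that switches the player's weapon to its WeaponType on overlap.
; On BeginPlay it sets its skeletal mesh to the assault rifle or shotgun to match that type.
; Overlap passes a DoOnce before casting to BP_Player and calling OnChangeWeapon, so any actor can consume the gate.
; Only a player ending overlap resets the gate, and the item stays in the world.
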(event EventBeginPlay
  (bind _skeletalmesh (Variables|Default|GetSkeletalMesh))
  (switch Utilities|FlowControl|Switch|SwitchonE_WeaponType (Variables|Default|GetWeaponType)
    (:NewEnumerator0
      (Components|SkeletalMesh|SetSkeletalMeshAsset _skeletalmesh "/Game/Props/MilitaryWeapSilver/Weapons/Assault_Rifle_A.Assault_Rifle_A"))
    (:NewEnumerator1
      (Components|SkeletalMesh|SetSkeletalMeshAsset _skeletalmesh "/Game/Props/MilitaryWeapSilver/Weapons/Shotgun_A.Shotgun_A"))))

(event Collision|EventActorBeginOverlap
  (params (OtherActor :type Actor%20Object%20Reference))
  (Utilities|FlowControl|DoOnce false
    (:Completed
      (bind _asbp_player (Utilities|Casting|CastToBP_Player OtherActor))
      (Default|OnChangeWeapon _asbp_player (Variables|Default|GetWeaponType)))))

(event Collision|EventActorEndOverlap
  (params (OtherActor :type Actor%20Object%20Reference))
  (Utilities|Casting|CastToBP_Player OtherActor)
  (Utilities|FlowControl|DoOnce false) ; enters at Reset
)

(fn ConstructionScript)